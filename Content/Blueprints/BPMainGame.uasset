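; BPMainGame runs a grid-based Snake game on the XZ plane, spawning the HUD, snake head, food and border walls.
; Tick uses a shrinking Delay as step timer, checking self, wall and food hits by location comparison, not physics.
; Eating adds score, a segment and speed; movement shifts segments back to front, with input gates allowing one turn per step.
; Death blanks the snake and shows game over; R opens a level-reload gate.
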(event `SpawnNewSnakePart`
  (params (SpawnLocation :type "Vector Structure") (IsHead :type Boolean))
  ;[1 1 1] SpawnNewSnakePart
  (bind _returnvalue (`|SpawnActorFromClass` "/Game/Blueprints/BPSnakeBodyPart.BPSnakeBodyPart_C" (`KismetMathLibrary.MakeTransform` SpawnLocation) "AlwaysSpawn" "OverrideRootScale" null null))
  (`PaperFlipbookComponent.SetFlipbook` (`/Game/Blueprints/BPSnakeBodyPart.PaperFlipbook` _returnvalue) (select `bool` IsHead :`false` "/Game/Flipbooks/YellowSquare_Flipbook.YellowSquare_Flipbook" :`true` "/Game/Flipbooks/RedSquare_Flipbook.RedSquare_Flipbook" :!type "PaperFlipbook Object Reference"))
  (`KismetArrayLibrary.Array_Add` (`self.SnakePartsArray`) _returnvalue)
  (set `/Game/Blueprints/BPSnakeBodyPart.IsHead` IsHead _returnvalue)
  (`self.K2_SetActorRotation` _returnvalue (`KismetMathLibrary.MakeRotator` 0.0 (select `int` (`KismetMathLibrary.RandomInteger` 3) :`0` 0.0 :`1` 90.0 :`2` 180.0 :`3` 270.0 :!type "Float (single-precision)")) false))

(event `SpawnFood`
  (bind _returnvalue (- (`self.ZMax`) 100.0))
  (bind _returnvalue_2 (- (`self.XMax`) 100.0))
  ;[1 1 1] SpawnFood
  (bind _returnvalue_3 (`|SpawnActorFromClass` "/Game/Blueprints/BPFood.BPFood_C" (`KismetMathLibrary.MakeTransform` (`KismetMathLibrary.MakeVector` (* (`.ReturnValue` (`KismetMathLibrary.FMod` (`KismetMathLibrary.RandomFloatInRange` (* _returnvalue_2 -1.0) _returnvalue_2) 100.0)) 100.0) 0.0 (* (`.ReturnValue` (`KismetMathLibrary.FMod` (`KismetMathLibrary.RandomFloatInRange` (* _returnvalue -1.0) _returnvalue) 100.0)) 100.0))) "AlwaysSpawn" "OverrideRootScale" null null))
  (set `self.FoodActorRef` _returnvalue_3))

(event `KillSnake`
  ;[1 1 1] KillSnake
  (set `self.IsDead` true)
  (for (_array_element _array_index) (`self.SnakePartsArray`)
    (`PaperFlipbookComponent.SetFlipbook` (`/Game/Blueprints/BPSnakeBodyPart.PaperFlipbook` _array_element) (select `bool` (== _array_index 0) :`false` "/Game/Flipbooks/Beath_Flipbook.Beath_Flipbook" :`true` "/Game/Flipbooks/Blank_Flipbook.Blank_Flipbook" :!type "PaperFlipbook Object Reference")))
  (`KismetSystemLibrary.Delay` 0.5)
  (for _array_element_2 (`self.SnakePartsArray`)
    (`PaperFlipbookComponent.SetFlipbook` (`/Game/Blueprints/BPSnakeBodyPart.PaperFlipbook` _array_element_2) "/Game/Flipbooks/Blank_Flipbook.Blank_Flipbook")))

(event `UpdateScore`
  (params (Value :type Integer))
  ;[1 1 1] UpdateScore
  (bind _output_get (set `self.Score` (+ Value (`self.Score`))))
  (`/Game/Blueprints/BPUIHud.UpdateScore` (`self.HUDRef`) _output_get))

(event `self.ReceiveBeginPlay`
  (bind (_remainder _returnvalue) (`KismetMathLibrary.FMod` (`self.XMax`) 50.0))
  (bind (_remainder_2 _returnvalue_2) (`KismetMathLibrary.FMod` (`self.ZMax`) 50.0))
  ;[1 1 1] InitializeGame
  (bind _returnvalue_3 (`|CreateWidget` "/Game/Blueprints/BPUIHud.BPUIHud_C"))
  (bind _output_get (set `self.HUDRef` _returnvalue_3))
  (`UserWidget.AddToViewport` _output_get 0)
  (switch `int` (`KismetMathLibrary.RandomInteger` 3)
    (:`0`
      (set `self.DirectionX` 1))
    (:`1`
      (set `self.DirectionX` -1))
    (:`2`
      (set `self.DirectionZ` 1))
    (:`3`
      (set `self.DirectionZ` -1)))
  (set `self.Delay` 0.2)
  (`KismetArrayLibrary.Array_Clear` (`self.SnakePartsArray`))
  (`self.SpawnNewSnakePart` (0.0 0.0 0.0) true)
  (`self.SpawnFood`)
  (for _index (range (* _returnvalue _returnvalue_2))
    (bind _returnvalue_4 (/ _index _returnvalue_2))
    (bind _returnvalue_5 (mod _index _returnvalue_2))
    (if (or (== _returnvalue_4 0) (== _returnvalue_4 (- _returnvalue 1)) (== _returnvalue_5 0) (== _returnvalue_5 (- _returnvalue_2 1)))
      (bind _returnvalue_6 (`|SpawnActorFromClass` "/Game/Blueprints/BPBlock.BPBlock_C" (`KismetMathLibrary.MakeTransform` (`KismetMathLibrary.MakeVector` (+ (* (`self.XMax`) -1.0) (* _returnvalue_4 100.0)) 0.0 (+ (* (`self.ZMax`) -1.0) (* _returnvalue_5 100.0)))) "AdjustIfPossibleButDontSpawnIfColliding" "OverrideRootScale" null null))
      (`KismetArrayLibrary.Array_Add` (`self.WallBlocksArray`) _returnvalue_6))))

(event `Key|R`
  (params (Key :type "Key Structure"))
  (:`Pressed`
    (goto _label :!via `Open`)))

(event `self.ReceiveTick`
  (params (DeltaSeconds :type "Float (single-precision)"))
  (bind _snakepartsarray (`self.SnakePartsArray`))
  (if (`self.IsDead`)
    (`/Engine/EditorBlueprintResources/StandardMacros.Gate` true :!label _label
      (:`Exit`
        (`/Engine/EditorBlueprintResources/StandardMacros.DoOnce` false
          (:`Completed`
            (`Widget.RemoveFromParent` (`self.HUDRef`))
            (bind _returnvalue (`GameplayStatics.GetCurrentLevelName` true))
            (`GameplayStatics.OpenLevel` (`KismetStringLibrary.Conv_StringToName` _returnvalue))))))
    (else
      (`KismetSystemLibrary.Delay` (`self.Delay`))
      (`|ExecutionSequence`
        (:`then_0`
          (for (_array_element _array_index) (`self.SnakePartsArray`) :!label _label_2
            (if (!= _array_index 0)
              (if (== (`self.K2_GetActorLocation` _array_element) (`self.K2_GetActorLocation` (`|GetArrayItem` (`self.SnakePartsArray`))))
                (`self.KillSnake`)
                (`/Game/Blueprints/BPUIHud.GameOverEvent` (`self.HUDRef`))
                (`self.BreakSelfCollisionSelfLoop`))))
          (for _array_element_2 (`self.WallBlocksArray`) :!label _label_3
            (if (== (`self.K2_GetActorLocation` _array_element_2) (`self.K2_GetActorLocation` (`|GetArrayItem` (`self.SnakePartsArray`))))
              (`self.KillSnake`)
              (`/Game/Blueprints/BPUIHud.GameOverEvent` (`self.HUDRef`))
              (`self.BreakWallCollisionTestLoop`))))
        (:`then_1`
          (if (not (`self.IsDead`))
            (`|ExecutionSequence`
              (:`then_0`
                (if (== (`self.K2_GetActorLocation` (`|GetArrayItem` (`self.SnakePartsArray`))) (`self.K2_GetActorLocation` (`self.FoodActorRef`)) :`ErrorTolerance` 1.0)
                  (`self.UpdateScore` (`/Game/Blueprints/BPFood.Score` (`self.FoodActorRef`)))
                  (`self.K2_DestroyActor` (`self.FoodActorRef`))
                  (`self.SpawnNewSnakePart` (`self.K2_GetActorLocation` (`|GetArrayItem` _snakepartsarray (`KismetArrayLibrary.Array_LastIndex` _snakepartsarray))))
                  (`self.SpawnFood`)
                  (set `self.Delay` (`KismetMathLibrary.FClamp` (+ (`self.Delay`) -0.01) 0.075 0.2))))
              (:`then_1`
                (`|ExecutionSequence`
                  (:`then_0`
                    (`/Engine/EditorBlueprintResources/StandardMacros.Gate` true :!label _label_4
                      (:`Exit`
                        (if (and (== (`self.DirectionZ`) 0) (`self.CanChangeDirection`))
                          (set `self.DirectionX` 0)
                          (set `self.DirectionZ` 1)
                          (set `self.CanChangeDirection` false :!label _label_5)))))
                  (:`then_1`
                    (`/Engine/EditorBlueprintResources/StandardMacros.Gate` true :!label _label_6
                      (:`Exit`
                        (if (and (== (`self.DirectionZ`) 0) (`self.CanChangeDirection`))
                          (set `self.DirectionX` 0)
                          (set `self.DirectionZ` -1)
                          (goto _label_5)))))
                  (:`then_2`
                    (`/Engine/EditorBlueprintResources/StandardMacros.Gate` true :!label _label_7
                      (:`Exit`
                        (if (and (== (`self.DirectionX`) 0) (`self.CanChangeDirection`))
                          (set `self.DirectionX` 1)
                          (set `self.DirectionZ` 0)
                          (goto _label_5)))))
                  (:`then_3`
                    (`/Engine/EditorBlueprintResources/StandardMacros.Gate` true :!label _label_8
                      (:`Exit`
                        (if (and (== (`self.DirectionX`) 0) (`self.CanChangeDirection`))
                          (set `self.DirectionX` -1)
                          (set `self.DirectionZ` 0)
                          (goto _label_5)))))
                  (:`then_4`
                    (for _index (range (`KismetArrayLibrary.Array_Length` (`self.SnakePartsArray`)))
                      (bind _returnvalue_2 (- (- (`KismetArrayLibrary.Array_Length` (`self.SnakePartsArray`)) 1) _index))
                      (if (`/Game/Blueprints/BPSnakeBodyPart.IsHead` (`|GetArrayItem` (`self.SnakePartsArray`) _returnvalue_2))
                        (bind _output (`|GetArrayItem` (`self.SnakePartsArray`) _returnvalue_2))
                        (`self.K2_AddActorWorldOffset` _output (`KismetMathLibrary.MakeVector` (`KismetMathLibrary.Conv_IntToDouble` (* (`self.DirectionX`) 100)) 0.0 (`KismetMathLibrary.Conv_IntToDouble` (* (`self.DirectionZ`) 100))) false false)
                        (else
                          (`self.K2_SetActorLocation` _output (`self.K2_GetActorLocation` (`|GetArrayItem` (`self.SnakePartsArray`) (- _returnvalue_2 1))) false false))))
                    (set `self.CanChangeDirection` true)))))))))))

(event `BreakSelfCollisionSelfLoop`
  (goto _label_2 :!via `Break`))

(event `BreakWallCollisionTestLoop`
  (goto _label_3 :!via `Break`))

(event `InputAction|SnakeUp`
  (params (Key :type "Key Structure"))
  (:`Pressed`
    (goto _label_4 :!via `Open`))
  (:`Released`
    (goto _label_4 :!via `Close`)))

(event `InputAction|SnakeDown`
  (params (Key :type "Key Structure"))
  (:`Pressed`
    (goto _label_6 :!via `Open`))
  (:`Released`
    (goto _label_6 :!via `Close`)))

(event `InputAction|SnakeRight`
  (params (Key :type "Key Structure"))
  (:`Pressed`
    (goto _label_7 :!via `Open`))
  (:`Released`
    (goto _label_7 :!via `Close`)))

(event `InputAction|SnakeLeft`
  (params (Key :type "Key Structure"))
  (:`Pressed`
    (goto _label_8 :!via `Open`))
  (:`Released`
    (goto _label_8 :!via `Close`)))

(fn `UserConstructionScript`)